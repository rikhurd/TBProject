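; BP_PlayerController is the player controller that turns Enhanced Input actions into pawn commands and mouse-driven turning.
; It adds the IMC_Player mapping context on BeginPlay and forwards move and interact actions to the controlled pawn as messages, leaving their behavior to the pawn.
; While the mouse movement mode action is active, it hides the cursor and feeds horizontal mouse movement into yaw, then shows the cursor again on completion.
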(event Input|EnhancedActionEvents|EnhancedInputActionIA_Move
  (params (ActionValue :type Vector%202D%20Structure) (ElapsedSeconds :type Float%20%28double-precision%29) (TriggeredSeconds :type Float%20%28double-precision%29) (InputAction :type Input%20Action%20Object%20Reference :default "/Game/Inputs/IA_Move.IA_Move"))
  (:Triggered
    (Class|BPIPlayerInput|PlayerMove(Message) (Pawn|GetControlledPawn) ActionValue)))

(event Input|EnhancedActionEvents|EnhancedInputActionIA_Interact
  (params (ActionValue :type Boolean) (ElapsedSeconds :type Float%20%28double-precision%29) (TriggeredSeconds :type Float%20%28double-precision%29) (InputAction :type Input%20Action%20Object%20Reference :default "/Game/Inputs/IA_Interact.IA_Interact"))
  (:Triggered
    (Class|BPIPlayerInput|PlayerInteract(Message) (Pawn|GetControlledPawn))))

(event Input|EnhancedActionEvents|EnhancedInputActionIA_MouseMovementMode
  (params (ActionValue :type Boolean) (ElapsedSeconds :type Float%20%28double-precision%29) (TriggeredSeconds :type Float%20%28double-precision%29) (InputAction :type Input%20Action%20Object%20Reference :default "/Game/Inputs/IA_MouseMovementMode.IA_MouseMovementMode"))
  (:Triggered
    (Class|PlayerController|AddYawInput (.x (Input|EnhancedActionValues|GetIA_MouseMovement))))
  (:Started
    (Variables|Default|SetbShowMouseCursor false))
  (:Completed
    (Variables|Default|SetbShowMouseCursor true)))

(event EventBeginPlay
  (Input|AddMappingContext (PlayerController|LocalPlayerSubsystems|GetEnhancedInputLocalPlayerSubsystem) "/Game/Inputs/IMC_Player.IMC_Player" 0 "(bIgnoreAllPressedKeysUntilRelease=True,bForceImmediately=False)"))

(fn ConstructionScript)