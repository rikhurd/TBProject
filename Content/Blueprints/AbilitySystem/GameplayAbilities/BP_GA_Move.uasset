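; BP_GA_Move is the move gameplay ability for tile-based characters, built on a C++ tile-targeting parent.
; AbilitySetup, called by that parent, finds a path from the owning character's current tile to the selected tile, stores it and returns whether it is non-empty.
; Activation only commits the ability's cost and prints whether that succeeded; this graph does not move the character along the path.
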(event Ability|EventActivateAbility
  ;[1 1 1] Commit subtracts whatever cost the ability has from the attribute set
  (bind _returnvalue (Ability|CommitAbility))
  (Development|PrintString (Utilities|String|Append "Ability commit success: " (Utilities|String|ToString(Boolean) _returnvalue))))

(event Ability|EventCommitExecute)

(fn AbilitySetup
  (params (SelectedTarget :type Actor%20Object%20Reference))
  (bind _astbcharacter_base (Utilities|Casting|CastToTBCharacterBase (Ability|GetOwningActorfromActorInfo)))
  (Variables|Default|SetOwningCharacter _astbcharacter_base)
  (Utilities|IsValid (Variables|/Script/TBS_Project.TBCharacterBase|GetCurrentTile _astbcharacter_base)
    (:Is%20Valid
      (bind _astile_base (Utilities|Casting|CastToTileBase SelectedTarget))
      (Utilities|IsValid _astile_base
        (:Is%20Valid
          (bind _returnvalue (Class|Pathfinding|FindPath (Variables|/Script/TBS_Project.TBCharacterBase|GetCurrentTile _astbcharacter_base) _astile_base))
          (bind _output_get (Variables|Default|SetAbilityPath _returnvalue))
          (return (Utilities|Array|IsNotEmpty _output_get)) ; This bool gets sent into Parent TargetTile func
        )))))