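; Player controller for a turn-based game with free and grid movement, routing Enhanced Input to the controlled pawn and game state.
; It creates the UI layout for pushing menu and combat layers, forwarding character selection to the current UI.
; Pathfinding between start and target tiles feeds instanced highlights on a spawned actor and gates placeholder teleport movement.
; Cursor-traced tile choices are passed to the selected character's gameplay ability.
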(event Custom|MoveCharacterOnGrid_1
  (params (TileToMove :type Tile%20Base%20Object%20Reference))
  (bind _returnvalue (Transformation|GetActorLocation TileToMove))
  ;[1 1 1] Placeholder character movement on Grid. PH now teleports actor to the location
  (if (and (Utilities|Array|ContainsItem (Variables|Default|GetPathFound) TileToMove) (Utilities|IsValid (Variables|Default|GetSelectedCharacter)))
    (Transformation|SetActorLocation (Variables|Default|GetSelectedCharacter) (Math|Vector|MakeVector (.x _returnvalue) (.y _returnvalue) 1e+02) false false)))

(event Input|EnhancedActionEvents|EnhancedInputActionIA_Move
  (params (ActionValue :type Vector%202D%20Structure) (ElapsedSeconds :type Float%20%28double-precision%29) (TriggeredSeconds :type Float%20%28double-precision%29) (InputAction :type Input%20Action%20Object%20Reference :default "/Game/Inputs/Actions/IA_Move.IA_Move"))
  ;[1 1 1] Handles moving in 3D free and when going to grid spawn new pawn and possess it uses this same system to move
  (Class|BPIPlayerInput|PlayerMove(Message) (Pawn|GetControlledPawn) ActionValue))

(event Input|EnhancedActionEvents|EnhancedInputActionIA_Interact
  (params (ActionValue :type Boolean) (ElapsedSeconds :type Float%20%28double-precision%29) (TriggeredSeconds :type Float%20%28double-precision%29) (InputAction :type Input%20Action%20Object%20Reference :default "/Game/Inputs/Actions/IA_Interact.IA_Interact"))
  ;[1 1 1] Handles moving in 3D free and when going to grid spawn new pawn and possess it uses this same system to move
  (Class|BPIPlayerInput|PlayerInteract(Message) (Pawn|GetControlledPawn)))

(event Input|EnhancedActionEvents|EnhancedInputActionIA_CameraRotation
  (params (ActionValue :type Float%20%28double-precision%29) (ElapsedSeconds :type Float%20%28double-precision%29) (TriggeredSeconds :type Float%20%28double-precision%29) (InputAction :type Input%20Action%20Object%20Reference :default "/Game/Inputs/Actions/IA_CameraRotation.IA_CameraRotation"))
  (Class|PlayerController|AddYawInput ActionValue))

(event Input|EnhancedActionEvents|EnhancedInputActionIA_CancelMovement
  (params (ActionValue :type Boolean) (ElapsedSeconds :type Float%20%28double-precision%29) (TriggeredSeconds :type Float%20%28double-precision%29) (InputAction :type Input%20Action%20Object%20Reference :default "/Game/Inputs/Actions/IA_CancelMovement.IA_CancelMovement"))
  (Variables|Default|SetPathfindingStartTileRef 0))

(event Input|EnhancedActionEvents|EnhancedInputActionIA_EndTurn
  (params (ActionValue :type Boolean) (ElapsedSeconds :type Float%20%28double-precision%29) (TriggeredSeconds :type Float%20%28double-precision%29) (InputAction :type Input%20Action%20Object%20Reference :default "/Game/Inputs/Actions/IA_EndTurn.IA_EndTurn"))
  (Class|BPIPlayerInput|PlayerEndTurn(Message) (Game|GetGameState)))

(event Input|EnhancedActionEvents|EnhancedInputActionIA_OpenMenu
  (params (ActionValue :type Boolean) (ElapsedSeconds :type Float%20%28double-precision%29) (TriggeredSeconds :type Float%20%28double-precision%29) (InputAction :type Input%20Action%20Object%20Reference :default "/Game/Inputs/Actions/IA_OpenMenu.IA_OpenMenu"))
  (bind _playeruilayout (Variables|Default|GetPlayerUILayout))
  (Utilities|FlowControl|FlipFlop
    (:A
      (Default|PushGameMenu _playeruilayout "/Game/Blueprints/UI/W_GameMenu.W_GameMenu_C"))
    (:B
      (Default|PopGameMenu _playeruilayout))))

(event EventBeginPlay
  (Input|AddMappingContext (PlayerController|LocalPlayerSubsystems|GetEnhancedInputLocalPlayerSubsystem) "/Game/Inputs/Mappings/IMC_Default_KBM.IMC_Default_KBM" 0 "(bIgnoreAllPressedKeysUntilRelease=True,bForceImmediately=False,bNotifyUserSettings=False)")
  ;[1 1 1] Create player UI Layout and make it into a variable that we can push widget stacks on
  (bind _returnvalue (UserInterface|CreateWidget "/Game/Blueprints/UI/W_UILayout.W_UILayout_C" self))
  (bind _output_get (Variables|Default|SetPlayerUILayout _returnvalue))
  (UserInterface|Viewport|AddtoViewport _output_get 0)
  (bind _returnvalue_2 (Game|SpawnActorfromClass "/Game/Blueprints/Grid/BP_TileHighlight.BP_TileHighlight_C" (Math|Transform|MakeTransform "0, 0, 0" "0, 0, 0" "1.000000,1.000000,1.000000") "Undefined" "OverrideRootScale" self 0))
  (Variables|Default|SetTileHighlightReference _returnvalue_2))

(event EventPathfindingStartTile
  (params (StartTile :type Tile%20Base%20Object%20Reference) (CharacterToMove :type Pawn%20Object%20Reference) (CharacterMovementRange :type Integer))
  ;[1 1 1] Check both start tile and end tile is set
  (Variables|Default|SetPathfindingStartTileRef StartTile))

(event EventPathfindingTargetTile
  (params (TargetTile :type Tile%20Base%20Object%20Reference))
  ;[1 1 1] Check both start tile and end tile is set
  (Variables|Default|SetPathfindingTargetTileRef TargetTile)
  (if (and (Utilities|IsValid (Variables|Default|GetPathfindingStartTileRef)) (Utilities|IsValid (Variables|Default|GetPathfindingTargetTileRef)))
    (bind _returnvalue (Class|Pathfinding|FindPath (Variables|Default|GetPathfindingStartTileRef) (Variables|Default|GetPathfindingTargetTileRef)))
    (bind _output_get (Variables|Default|SetPathFound _returnvalue))
    (if (Utilities|Array|IsNotEmpty _output_get)
      (for _array_element _output_get
        (bind _returnvalue_2 (Components|InstancedStaticMesh|AddInstance (Variables|/Game/Blueprints/Grid/BP_TileHighlight.BP_TileHighlight_C|GetInstancedHighlight (Variables|Default|GetTileHighlightReference)) (Math|Transform|MakeTransform (Math|Vector|MakeVector (.x (Transformation|GetActorLocation _array_element)) (.y (Transformation|GetActorLocation _array_element)) 16.0) "0, 0, 0" "1.000000,1.000000,1.000000") true))
        (Utilities|Array|AddUnique (Variables|Default|GetTileHighlightInstancesId) _returnvalue_2)))))

(event EventMoveTileHighlight
  (params (Location :type Vector :default "0, 0, 0"))
  (Rendering|SetActorHiddenInGame (Variables|Default|GetTileHighlightReference) true)
  (Transformation|SetActorLocation (Variables|Default|GetTileHighlightReference) Location false false)
  (Rendering|SetActorHiddenInGame (Variables|Default|GetTileHighlightReference) false))

(event EventHideTileHighlight
  ;[1 1 1] Hides placeholder highlight when it is not needed
  (Rendering|SetActorHiddenInGame (Variables|Default|GetTileHighlightReference) true)
  (if (Utilities|Array|IsNotEmpty (Variables|Default|GetTileHighlightInstancesId))
    (CallFunction|RemoveHighlightInstances)))

(event EventPlayerSelect
  (params (SelectedCharacter :type TB%20Character%20Base%20Object%20Reference))
  (bind _current_ui (Variables|Default|GetCurrent%20UI))
  (Variables|Default|SetSelectedCharacter SelectedCharacter)
  (Utilities|IsValid _current_ui
    (:Is%20Valid
      (Class|BPIPlayerInput|PlayerSelect(Message) _current_ui (Variables|Default|GetSelectedCharacter)))))

(event EventPlayerCurrentUI
  (params (CurrentUI :type Common%20Activatable%20Widget%20Object%20Reference))
  (Variables|Default|SetCurrent%20UI CurrentUI))

(event EventCombatModeInit
  (Default|PushGameLayer (Variables|Default|GetPlayerUILayout) "/Game/Blueprints/UI/W_GameLayer.W_GameLayer_C"))

(event Input|EnhancedActionEvents|EnhancedInputActionIA_Choose
  (params (ActionValue :type Boolean) (ElapsedSeconds :type Float%20%28double-precision%29) (TriggeredSeconds :type Float%20%28double-precision%29) (InputAction :type Input%20Action%20Object%20Reference :default "/Game/Inputs/Actions/IA_Choose.IA_Choose"))
  (bind _selectedcharacter (Variables|Default|GetSelectedCharacter))
  ;[1 1 1] Placeholder for later
  (Utilities|IsValid _selectedcharacter
    (:Is%20Valid
      (switch Utilities|FlowControl|Switch|SwitchonEAbilityTargetSelectType (Variables|Default|GetTileSelectType)
        (:Any
          (bind _output_get (CallFunction|NewFunction))
          (Class|TBAbilityInterface|AbilityTargetTile(Message) (.ReturnValue (Ability|GameplayAbility|GetGameplayAbilityfromSpecHandle (Class|TBCharacterBase|GetAbilitySystemComponent _selectedcharacter) (Variables|Default|GetCurrentAbilityHandler))) _output_get))))))

(event EventSelectTile
  (params (AbilityHandler :type Gameplay%20Ability%20Spec%20Handle%20Structure) (TileSelectType :type EAbilityTargetSelectType%20Enum :default "Any"))
  (Variables|Default|SetCurrentAbilityHandler AbilityHandler)
  (Variables|Default|SetTileSelectType TileSelectType)
  (Variables|Default|SetTileSelected true))

(fn ConstructionScript)

(fn RemoveHighlightInstances
  (bind _tilehighlightinstancesid (Variables|Default|GetTileHighlightInstancesId))
  (Class|InstancedStaticMeshComponent|RemoveInstances (Variables|/Game/Blueprints/Grid/BP_TileHighlight.BP_TileHighlight_C|GetInstancedHighlight (Variables|Default|GetTileHighlightReference)) _tilehighlightinstancesid)
  (Utilities|Array|Clear _tilehighlightinstancesid))

(fn ClearPath
  (params (TargetArray :type Array%20of%20Tile%20Base%20Object%20References))
  (Variables|Default|SetPathfindingStartTileRef 0)
  (Utilities|Array|Clear TargetArray))

(fn GetTile)

(fn NewFunction
  (bind _array (Utilities|Array|MakeArray "ObjectTypeQuery7"))
  (bind (_hitresult _returnvalue) (Class|PlayerController|GetHitResultUnderCursorforObjects _array false))
  (if (and (Variables|Default|GetTileSelected) _returnvalue)
    (bind _output_get (Variables|Default|SetSelectedTile (.HitActor (Collision|BreakHitResult _hitresult)))))
  (return _output_get))