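; BP_PlayerCamera is a player camera actor that moves in response to movement input.
; The PlayerMove event maps input X to the actor's forward vector and Y to its right vector, then feeds the sum to the movement component.
; The construction script sets the camera's world rotation from the CameraRotation variable, so movement follows the actor's facing rather than the camera's angle.
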(event EventPlayerMove
  (params (MovementInput :type Vector%202D%20Structure))
  (Class|PawnMovementComponent|AddInputVector (Variables|Default|GetMovementComponent) (+ (* (.x MovementInput) (Transformation|GetActorForwardVector)) (* (.y MovementInput) (Transformation|GetActorRightVector))) false))

(fn ConstructionScript
  (Transformation|SetWorldRotation (Variables|Default|GetCamera) (Variables|Default|GetCameraRotation) false false))