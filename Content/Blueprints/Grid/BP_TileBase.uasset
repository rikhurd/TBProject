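; BP_TileBase is a grid tile actor that holds an index and a walkable state.
; On BeginPlay it writes its X,Y index into a coordinate text component.
; As placeholder test tooling, hovering the cursor with Shift held calls ToggleWalkable to paint impassable walls.
; ToggleWalkable flips Walkable and sets the Plane's hidden state to match, so the plane shows only on unwalkable tiles.
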(event EventBeginPlay
  (bind _index (Variables|Default|GetIndex))
  (bind (_x _y) (Utilities|Struct|BreakIntPoint _index))
  ;[1 1 1] Shows tile coordinates or index in the grid
  (Rendering|Components|TextRender|SetText (Variables|Default|GetTileCoordinates) (Utilities|Text|ToText(String) (Utilities|String|Append (Utilities|String|ToString(Text) (Utilities|Text|ToText(Integer) _x)) "," (Utilities|String|ToString(Text) (Utilities|Text|ToText(Integer) _y))))))

(event MouseInput|EventActorBeginCursorOver
  ;[1 1 1] Placeholder for painting impassable walls on the grid for testing
  (if (Class|KismetInputLibrary|ModifierKeysStateIsShiftDown (Class|KismetInputLibrary|GetModifierKeysState))
    (CallFunction|ToggleWalkable)))

(fn ConstructionScript)

(fn ToggleWalkable
  (bind _plane (Variables|Default|GetPlane))
  (if (Variables|Default|GetWalkable)
    (bind _output_get (Variables|Default|SetWalkable false))
    (Development|SetHiddeninGame _plane _output_get false)
    (else
      (bind _output_get_2 (Variables|Default|SetWalkable true))
      (Development|SetHiddeninGame _plane _output_get_2 false))))