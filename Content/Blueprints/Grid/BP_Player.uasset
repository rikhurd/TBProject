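; BP_Player is the player character, which moves relative to its facing, interacts with actors and has hooks for grid battle and exploration modes.
; IA_Interact sends PlayerInteractMessage to the last overlapped actor, cleared on any overlap end.
; The construction script binds both mode-start dispatchers.
; Battle start stores the grid reference and binds an OnClicked event; click handling only prints debug text, and exploration start is empty.
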(event Custom|BattleOnClicked
  (params (TouchedActor :type Actor%20Object%20Reference) (ButtonPressed :type Key%20Structure :default "None"))
  (Development|PrintString (Utilities|GetDisplayName TouchedActor)))

(event Input|EnhancedActionEvents|EnhancedInputActionIA_Interact
  (params (ActionValue :type Boolean) (ElapsedSeconds :type Float%20%28double-precision%29) (TriggeredSeconds :type Float%20%28double-precision%29) (InputAction :type Input%20Action%20Object%20Reference :default "/Game/Inputs/IA_Interact.IA_Interact"))
  (bind _overlappingactorref (Variables|Default|GetOverlappingActorRef))
  (:Triggered
    (Utilities|IsValid _overlappingactorref
      (:Is%20Valid
        (Class|BPIPlayerInput|PlayerInteract(Message) _overlappingactorref self)))))

(event EventBeginPlay)

(event Collision|EventActorBeginOverlap
  (params (OtherActor :type Actor%20Object%20Reference))
  (Variables|Default|SetOverlappingActorRef OtherActor))

(event EventTick
  (params (DeltaSeconds :type Float%20%28single-precision%29)))

(event EventPlayerMove
  (params (MovementInput :type Vector%202D%20Structure))
  (Class|PawnMovementComponent|AddInputVector (Variables|Character|GetCharacterMovement) (+ (* (.x MovementInput) (Transformation|GetActorForwardVector)) (* (.y MovementInput) (Transformation|GetActorRightVector))) false))

(event Collision|EventActorEndOverlap
  (params (OtherActor :type Actor%20Object%20Reference))
  (Variables|Default|SetOverlappingActorRef 0))

(fn ConstructionScript
  (EventDispatchers|BindEventtoPlayerBattleModeStartDispatcher (EventDispatchers|CreateEvent :!event PlayerBattleModeStart))
  (EventDispatchers|BindEventtoPlayerExplorationModeStartDispatcher (EventDispatchers|CreateEvent :!event PlayerExplorationmodeStart)))

(fn PlayerBattleModeStart
  (params (GridRef :type BP%20Grid%20Object%20Reference))
  (Variables|Default|SetGrid%20Ref GridRef)
  (Development|PrintString "Hello")
  (EventDispatchers|BindEventtoOnClicked (EventDispatchers|CreateEvent :!event Custom|BattleOnClicked)))

(fn PlayerExplorationmodeStart)