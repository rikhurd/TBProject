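; BP_TileCollision is a grid tile actor that drives the tile highlight when the cursor hovers over it.
; It caches BP_GameMode on BeginPlay and, on each hover event, looks up the PlayerController of the current PlayerTurn.
; Cursor enter tells that controller to move the highlight to the tile's location, and cursor exit tells it to hide the highlight.
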(event EventBeginPlay
  (bind _asbp_game_mode (Utilities|Casting|CastToBP_GameMode (Game|GetGameMode)))
  (Variables|Default|SetGameModeRef _asbp_game_mode))

(event MouseInput|EventActorBeginCursorOver
  (bind _gamemoderef (Variables|Default|GetGameModeRef))
  (bind _playerturn (Variables|/Game/Blueprints/GameControllers/BP_GameMode.BP_GameMode_C|GetPlayerTurn _gamemoderef))
  (Utilities|IsValid (.playercontroller _playerturn)
    (:Is%20Valid
      (bind _asbp_player_controller (Utilities|Casting|CastToBP_PlayerController (.playercontroller _playerturn)))
      (Class|BPIGridMovement|MoveTileHighlight(Message) _asbp_player_controller (Transformation|GetActorLocation)))))

(event MouseInput|EventActorEndCursorOver
  (bind _gamemoderef (Variables|Default|GetGameModeRef))
  (bind _playerturn (Variables|/Game/Blueprints/GameControllers/BP_GameMode.BP_GameMode_C|GetPlayerTurn _gamemoderef))
  (Utilities|IsValid (.playercontroller _playerturn)
    (:Is%20Valid
      (bind _asbp_player_controller (Utilities|Casting|CastToBP_PlayerController (.playercontroller _playerturn)))
      (Class|BPIGridMovement|HideTileHighlight(Message) _asbp_player_controller))))

(fn ConstructionScript)