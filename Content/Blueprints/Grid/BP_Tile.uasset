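; BP_Tile is a grid tile actor that highlights itself while the mouse cursor is over it.
; On BeginPlay it binds the begin and end cursor-over events and stores the mesh's slot 0 material in a Material variable.
; Hovering sets M_MouseOverTile as both overlay and slot 0 material.
; Leaving sets both from the BP_Tile class defaults rather than reading the stored instance value.
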(event Custom|OnBeginCursorOver_Event
  (params (TouchedActor :type Actor%20Object%20Reference))
  (Rendering|Material|SetOverlayMaterial (Variables|Default|GetStaticMesh) "/Game/Materials/M_MouseOverTile.M_MouseOverTile" :!class /Script/Engine.MeshComponent)
  (Rendering|Material|SetMaterial (Variables|Default|GetStaticMesh) 0 "/Game/Materials/M_MouseOverTile.M_MouseOverTile"))

(event Custom|OnEndCursorOver_Event
  (params (TouchedActor :type Actor%20Object%20Reference))
  (bind _material (Utilities|GetClassDefaults "BP_Tile_C"))
  (Rendering|Material|SetOverlayMaterial (Variables|Default|GetStaticMesh) _material :!class /Script/Engine.MeshComponent)
  (Rendering|Material|SetMaterial (Variables|Default|GetStaticMesh) 0 _material))

(event EventBeginPlay
  (EventDispatchers|BindEventtoOnBeginCursorOver (delegate Custom|OnBeginCursorOver_Event))
  (EventDispatchers|AssignOnEndCursorOver (delegate Custom|OnEndCursorOver_Event))
  (Variables|Default|SetMaterial (Rendering|Material|GetMaterial (Variables|Default|GetStaticMesh) 0)))

(fn ConstructionScript)