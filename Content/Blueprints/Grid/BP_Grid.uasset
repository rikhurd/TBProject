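; BP_Grid is a grid actor that generates a tiled floor and a random room definition when play begins.
; It rolls a room type and one to four doors from the GameMode's random stream and stores them in a room struct.
; A 2D grid macro centred on the actor then adds an instanced floor mesh per cell, records its location and coordinates in a tile array indexed by instance, and spawns a tile collision actor there.
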(event EventBeginPlay
  (bind _asbp_game_mode (Utilities|Casting|CastToBP_GameMode (Game|GetGameMode)))
  (Variables|Default|SetGameModeRef _asbp_game_mode)
  (CallFunction|GridConstruction))

(fn ConstructionScript)

(fn MakeRoomStructure
  (bind _gamemoderef (Variables|Default|GetGameModeRef))
  (bind _stream (Variables|/Game/Blueprints/GameControllers/BP_GameMode.BP_GameMode_C|GetStream _gamemoderef))
  (bind _returnvalue (Math|Random|RandomIntegerinRangefromStream 0 3 _stream))
  (Variables|Default|SetfRoomRef (Utilities|Struct|MakeF_Room (Utilities|Enum|ByteToEnumE_RoomTypes (Math|Conversions|ToByte(Integer) _returnvalue)) (+ _returnvalue 1))))

(fn SpawnGrid
  (bind _gridtilecount (Variables|Default|GetGridTileCount))
  (bind _gridtilecount_2 (Variables|Default|GetGridTileCount))
  (bind _gridtilecount_3 (Variables|Default|GetGridTileCount))
  (Utilities|Array|Resize (Variables|Default|GetF%20TileArray) (* (.x _gridtilecount_2) (.y _gridtilecount_2)))
  (bind (_current_point _total_points _0_1_phase _poly_center _x_row _y_row) (Utilities|2DGridExecutionMacroOwn (Variables|Default|GetGridSnapValue) (Transformation|GetActorLocation) (.x _gridtilecount_3) (.y _gridtilecount_3))
    (:Per%20Poly%20Execution
      (bind _returnvalue (Components|InstancedStaticMesh|AddInstance (Variables|Default|GetFloorMesh) (Math|Transform|MakeTransform _poly_center "0, 0, 0" "1.000000,1.000000,1.000000") true))
      (Utilities|Array|SetArrayElem (Variables|Default|GetF%20TileArray) _returnvalue (Utilities|Struct|MakeF_Tile _returnvalue 0 "NewEnumerator0" _poly_center _x_row _y_row (.X (Utilities|GetXYfromIndex _returnvalue (.x _gridtilecount) (.y _gridtilecount))) (.Y (Utilities|GetXYfromIndex _returnvalue (.x _gridtilecount) (.y _gridtilecount)))))
      (bind _returnvalue_2 (Game|SpawnActorfromClass "/Game/Blueprints/Grid/BP_TileCollision.BP_TileCollision_C" (Math|Transform|MakeTransform _poly_center "0, 0, 0" "1.000000,1.000000,1.000000") "Undefined" 0 0))
      (Utilities|Array|Add (Variables|Default|GetTileCollisionArray) _returnvalue_2))))

(fn GridConstruction
  (CallFunction|MakeRoomStructure)
  (CallFunction|SpawnGrid))