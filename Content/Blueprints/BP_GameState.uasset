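; Game State that tracks whether play is in Exploration or Battle mode and announces mode changes through event dispatchers.
; The Construction Script binds the dispatcher handlers, and SetGameStateMode fires the matching start dispatcher, passing a grid reference for battle.
; Battle setup stores the grid, disables input and movement for players in PlayerArray, and forwards the grid through each BP_Player's dispatcher.
; Exploration start only prints a message, with no restoration of input.
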(event Custom|Battle%20Mode%20Start
  (params (GridRef :type BP%20Grid%20Object%20Reference))
  (CallFunction|SetupBattleMode GridRef)
  (Development|PrintString "Battle mode started"))

(event Custom|Exploration%20Mode%20Start
  (Development|PrintString "Exploration mode started"))

(event EventBeginPlay)

(fn ConstructionScript
  (EventDispatchers|BindEventtoChangeGameStateModeDispatcher (EventDispatchers|CreateEvent :!event SetGameStateMode))
  (EventDispatchers|BindEventtoBattleModeStartDispatcher (EventDispatchers|CreateEvent :!event Custom|Battle%20Mode%20Start))
  (EventDispatchers|BindEventtoExplorationModeStartDispatcher (EventDispatchers|CreateEvent :!event Custom|Exploration%20Mode%20Start)))

(fn GetGameStateMode
  (return (Variables|Default|GetGameStateMode)))

(fn SetGameStateMode
  (params (GameStateMode :type E_GameStateModes%20Enum :default "NewEnumerator0") (GridRef :type BP%20Grid%20Object%20Reference))
  (bind _output_get (Variables|Default|SetGameStateMode GameStateMode))
  (switch Utilities|FlowControl|Switch|SwitchonE_GameStateModes _output_get
    (:NewEnumerator0
      (Default|CallExplorationModeStartDispatcher))
    (:NewEnumerator1
      (Default|CallBattleModeStartDispatcher GridRef))))

(fn SetupBattleMode
  (params (GridRef :type BP%20Grid%20Object%20Reference))
  (LocalVariables|SetGridReference GridRef)
  (for _array_element (Variables|Default|GetPlayerArray)
    (Input|DisableInput (PlayerState|GetPawn _array_element) (Game|GetPlayerController _array_element))
    (Input|SetIgnoreMoveInput (Game|GetPlayerController _array_element) true)
    (bind _asbp_player (Utilities|Casting|CastToBP_Player (PlayerState|GetPawn _array_element)))
    (Default|CallPlayerBattleModeStartDispatcher _asbp_player (LocalVariables|GetGridReference))))