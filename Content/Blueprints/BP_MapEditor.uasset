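; BP_MapEditor is a Blueprint that, as it stands, only reports the size of a linked floor mesh.
; Its Construction Script reads the local bounds of LinkedFloorRef's StaticMeshComponent and prints the min and max coordinates as one appended string.
; Unconnected nodes for mesh section extraction, world scale and actor bounds remain in the graph, and the Event Graph holds only disabled default events.
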(event EventBeginPlay)

(event Collision|EventActorBeginOverlap
  (params (OtherActor :type Actor%20Object%20Reference)))

(event EventTick
  (params (DeltaSeconds :type Float%20%28single-precision%29)))

(fn ConstructionScript
  (bind _linkedfloorref (Variables|Default|GetLinkedFloorRef))
  (bind _staticmeshcomponent (Variables|/Script/Engine.StaticMeshActor|GetStaticMeshComponent _linkedfloorref))
  (bind (_min _max) (Components|StaticMesh|GetLocalBounds _staticmeshcomponent))
  (Development|PrintString (Utilities|String|Append (Utilities|String|ToString(Float) (.x _min)) (Utilities|String|ToString(Float) (.y _min)) (Utilities|String|ToString(Float) (.z _min)) (Utilities|String|ToString(Float) (.x _max)) (Utilities|String|ToString(Float) (.y _max)) (Utilities|String|ToString(Float) (.z _max)))))