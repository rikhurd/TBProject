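; Turn-based game state that manages the turn timer through its PlayerEndTurn event.
; PlayerEndTurn clears the timer if it is active, otherwise it starts a looping timer by event and stores the handle.
; When a timer starts, it passes the handle and duration to each PlayerArray entry's player controller, which relays them to the game UI for display.
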(event EventPlayerEndTurn
  (if (Utilities|Time|IsTimerActivebyHandle (Variables|Default|GetTimerHandle))
    (Utilities|Time|ClearandInvalidateTimerbyHandle (Variables|Default|GetTimerHandle))
    (else
      (bind _returnvalue (Utilities|Time|SetTimerbyEvent (EventDispatchers|CreateEvent :!event ProgressCombatAbilities) (Variables|Default|GetTime) true))
      (Variables|Default|SetTimerHandle _returnvalue)
      (for _array_element (Variables|Default|GetPlayerArray self)
        ;[1 1 1] Send Time and Handler to Player Controller which gives it to the GameUI which shows time for the turn
        (Class|BPIPlayerInput|PlayerTurnTimer(Message) (Game|GetPlayerController _array_element) _returnvalue (Variables|Default|GetTime))))))

(fn ConstructionScript)