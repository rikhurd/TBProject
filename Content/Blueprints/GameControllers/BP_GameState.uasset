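; Game state that switches the game between Exploration (free movement) and grid-based Battle modes through event dispatchers bound in the construction script.
; Battle start stores the grid manager, disables each player's input and notifies their character, currently passing only the first player's controller.
; Exploration start only prints a message, so input is not restored here.
; EndTurn refreshes the character list, messages every character and increments a tick counter.
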(event Custom|Battle%20Mode%20Start
  (params (GridRef :type Grid%20Manager%20Object%20Reference))
  ;[1 1 1] Call when Battle mode starts and change from free movement to grid movement
  (CallFunction|SetupBattleMode GridRef)
  (Development|PrintString "Battle mode started"))

(event Custom|Exploration%20Mode%20Start
  ;[1 1 1] Call when Exploration mode starts and change from grid movement to free movement
  (Development|PrintString "Exploration mode started"))

(event EventBeginPlay
  (CallFunction|GetCharacters))

(event EventEndTurn
  (bind _charactersarray (CallFunction|GetCharacters))
  (for _array_element _charactersarray
    (Class|BPIGameInterface|EndTurn(Message) _array_element))
  (bind _result (Math|Integer|IncrementInt (Variables|Default|GetTickCount))
    (:%20%20
      (Variables|Default|SetTickCount _result))))

(fn ConstructionScript
  (EventDispatchers|BindEventtoChangeGameStateModeDispatcher (EventDispatchers|CreateEvent :!event SetGameStateMode))
  (EventDispatchers|BindEventtoBattleModeStartDispatcher (EventDispatchers|CreateEvent :!event Custom|Battle%20Mode%20Start))
  (EventDispatchers|BindEventtoExplorationModeStartDispatcher (EventDispatchers|CreateEvent :!event Custom|Exploration%20Mode%20Start)))

(fn GetGameStateMode
  (return (Variables|Default|GetGameStateMode)))

(fn SetGameStateMode
  (params (GameStateMode :type E_GameStateModes%20Enum :default "NewEnumerator0") (GridRef :type Grid%20Manager%20Object%20Reference))
  (bind _output_get (Variables|Default|SetGameStateMode GameStateMode))
  (switch Utilities|FlowControl|Switch|SwitchonE_GameStateModes _output_get
    (:NewEnumerator0
      (Default|CallExplorationModeStartDispatcher))
    (:NewEnumerator1
      (Default|CallBattleModeStartDispatcher GridRef))))

(fn SetupBattleMode
  (params (GridRef :type Grid%20Manager%20Object%20Reference))
  (bind _playerarray (Variables|Default|GetPlayerArray))
  ;[1 1 1] Sets up Battle mode for the game by removing free movement and calling Battle mode setup on characters too
  (LocalVariables|SetGridManagerRef GridRef)
  (for _array_element _playerarray
    (Input|DisableInput (PlayerState|GetPawn _array_element) (Game|GetPlayerController _array_element))
    (Input|SetIgnoreMoveInput (Game|GetPlayerController _array_element) true)
    (bind _asbp_character_base (Utilities|Casting|CastToBP_CharacterBase (PlayerState|GetPawn _array_element)))
    (Default|CallPlayerBattleModeStartDispatcher _asbp_character_base (LocalVariables|GetGridManagerRef) (Game|GetPlayerController (Utilities|Array|Get(acopy) _playerarray)))))

(fn GetCharacters
  (bind _outactors (Actor|GetAllActorsOfClass "/Game/Blueprints/Player/BP_CharacterBase.BP_CharacterBase_C"))
  (bind _output_get (Variables|Default|SetCharactersArray _outactors))
  (return _output_get))