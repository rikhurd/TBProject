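; Player controller for a grid-based tactics game that routes Enhanced Input to the controlled pawn and game state, and manages tile selection and movement.
; Start and target tile events feed a C++ A* Pathfinding actor, whose path is reversed and trimmed to the character's movement range.
; A spawned BP_TileHighlight shows the hovered tile and draws the path as instanced meshes.
; Placeholder movement teleports the selected character along valid paths and reports the move cost.
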(event Input|EnhancedActionEvents|EnhancedInputActionIA_Move
  (params (ActionValue :type Vector%202D%20Structure) (ElapsedSeconds :type Float%20%28double-precision%29) (TriggeredSeconds :type Float%20%28double-precision%29) (InputAction :type Input%20Action%20Object%20Reference :default "/Game/Inputs/IA_Move.IA_Move"))
  ;[1 1 1] Handles moving in 3D free and when going to grid spawn new pawn and possess it uses this same system to move
  (:Triggered
    (Class|BPIPlayerInput|PlayerMove(Message) (Pawn|GetControlledPawn) ActionValue)))

(event Input|EnhancedActionEvents|EnhancedInputActionIA_Interact
  (params (ActionValue :type Boolean) (ElapsedSeconds :type Float%20%28double-precision%29) (TriggeredSeconds :type Float%20%28double-precision%29) (InputAction :type Input%20Action%20Object%20Reference :default "/Game/Inputs/IA_Interact.IA_Interact"))
  (:Triggered
    (Class|BPIPlayerInput|PlayerInteract(Message) (Pawn|GetControlledPawn))))

(event Input|EnhancedActionEvents|EnhancedInputActionIA_CameraRotation
  (params (ActionValue :type Float%20%28double-precision%29) (ElapsedSeconds :type Float%20%28double-precision%29) (TriggeredSeconds :type Float%20%28double-precision%29) (InputAction :type Input%20Action%20Object%20Reference :default "/Game/Inputs/IA_CameraRotation.IA_CameraRotation"))
  (:Triggered
    (Class|PlayerController|AddYawInput ActionValue)))

(event Input|EnhancedActionEvents|EnhancedInputActionIA_CancelMovement
  (params (ActionValue :type Boolean) (ElapsedSeconds :type Float%20%28double-precision%29) (TriggeredSeconds :type Float%20%28double-precision%29) (InputAction :type Input%20Action%20Object%20Reference :default "/Game/Inputs/IA_CancelMovement.IA_CancelMovement"))
  (:Triggered
    (Variables|Default|SetPathfindingStartTileRef 0)))

(event Input|EnhancedActionEvents|EnhancedInputActionIA_EndTurn
  (params (ActionValue :type Boolean) (ElapsedSeconds :type Float%20%28double-precision%29) (TriggeredSeconds :type Float%20%28double-precision%29) (InputAction :type Input%20Action%20Object%20Reference :default "/Game/Inputs/IA_EndTurn.IA_EndTurn"))
  (:Triggered
    (Class|BPIGameInterface|EndTurn(Message) (Game|GetGameState))))

(event EventBeginPlay
  (Input|AddMappingContext (PlayerController|LocalPlayerSubsystems|GetEnhancedInputLocalPlayerSubsystem) "/Game/Inputs/IMC_Player.IMC_Player" 0 "(bIgnoreAllPressedKeysUntilRelease=True,bForceImmediately=False)")
  (bind _returnvalue (Game|SpawnActorfromClass "/Game/Blueprints/Grid/BP_TileHighlight.BP_TileHighlight_C" (Math|Transform|MakeTransform "0, 0, 0" "0, 0, 0" "1.000000,1.000000,1.000000") "Undefined" self 0))
  (Variables|Default|SetTileHighlightReference _returnvalue))

(event EventPathfindingStartTile
  (params (StartTile :type Tile%20Base%20Object%20Reference) (CharacterToMove :type Pawn%20Object%20Reference) (CharacterMovementRange :type Integer))
  (Variables|Default|SetPathfindingStartTileRef StartTile)
  (Variables|Default|SetCharacterMovementRange CharacterMovementRange)
  (Variables|Default|SetSelectedCharacter CharacterToMove) ; We get character to move because later it's meant to have multiple movable characters
  (if (and (Utilities|IsValid (Variables|Default|GetPathfindingStartTileRef)) (Utilities|IsValid (Variables|Default|GetPathfindingTargetTileRef)))
    (if (Utilities|IsValid (Variables|Default|GetPathfinderRef)) :!label _label
      (bind _filteredarray (CallFunction|FindPath))
      (for _array_element _filteredarray
        (bind _returnvalue (Components|InstancedStaticMesh|AddInstance (Variables|/Game/Blueprints/Grid/BP_TileHighlight.BP_TileHighlight_C|GetInstancedHighlight (Variables|Default|GetTileHighlightReference)) (Math|Transform|MakeTransform (Transformation|GetActorLocation _array_element) "0, 0, 0" "1.000000,1.000000,1.000000") true))
        (Utilities|Array|AddUnique (Variables|Default|GetTileHighlightInstancesId) _returnvalue))
      (else
        (CallFunction|GetPathfinderActor)
        (goto _label)))))

(event EventPathfindingTargetTile
  (params (TargetTile :type Tile%20Base%20Object%20Reference))
  (Variables|Default|SetPathfindingTargetTileRef TargetTile)
  (if (and (Utilities|IsValid (Variables|Default|GetPathfindingStartTileRef)) (Utilities|IsValid (Variables|Default|GetPathfindingTargetTileRef)))
    (if (Utilities|IsValid (Variables|Default|GetPathfinderRef)) :!label _label
      (bind _filteredarray (CallFunction|FindPath))
      (for _array_element _filteredarray
        (bind _returnvalue (Components|InstancedStaticMesh|AddInstance (Variables|/Game/Blueprints/Grid/BP_TileHighlight.BP_TileHighlight_C|GetInstancedHighlight (Variables|Default|GetTileHighlightReference)) (Math|Transform|MakeTransform (Transformation|GetActorLocation _array_element) "0, 0, 0" "1.000000,1.000000,1.000000") true))
        (Utilities|Array|AddUnique (Variables|Default|GetTileHighlightInstancesId) _returnvalue))
      (else
        (CallFunction|GetPathfinderActor)
        (goto _label)))))

(event EventMoveTileHighlight
  (params (Location :type Vector :default "0, 0, 0"))
  (Rendering|SetActorHiddenInGame (Variables|Default|GetTileHighlightReference) true)
  (Transformation|SetActorLocation (Variables|Default|GetTileHighlightReference) Location false false)
  (Rendering|SetActorHiddenInGame (Variables|Default|GetTileHighlightReference) false))

(event EventHideTileHighlight
  (Rendering|SetActorHiddenInGame (Variables|Default|GetTileHighlightReference) true)
  (if (Utilities|Array|IsNotEmpty (Variables|Default|GetTileHighlightInstancesId))
    (CallFunction|RemoveHighlightInstances)))

(event EventMoveCharacteronGrid
  (params (TileToMove :type Tile%20Base%20Object%20Reference) (MoveCost :type Integer))
  (bind _returnvalue (Transformation|GetActorLocation TileToMove))
  (bind _selectedcharacter (Variables|Default|GetSelectedCharacter))
  ;[1 1 1] Placeholder character movement on Grid. PH now teleports actor to the location
  (if (and (Utilities|Array|ContainsItem (Variables|Default|GetPathFound) TileToMove) (Utilities|IsValid (Variables|Default|GetSelectedCharacter)))
    (Transformation|SetActorLocation _selectedcharacter (Math|Vector|MakeVector (.x _returnvalue) (.y _returnvalue) 1e+02) false false)
    (Class|BPIGridMovement|MoveCharacteronGrid(Message) _selectedcharacter TileToMove (+ (Utilities|Array|FindItem (Variables|Default|GetPathFound) TileToMove) 1))
    (CallFunction|ClearPath)))

(fn ConstructionScript)

(fn GetPathfinderActor
  (bind _returnvalue (Actor|GetActorOfClass "/Script/TBS_Project.Pathfinding"))
  (Utilities|IsValid _returnvalue
    (:Is%20Valid
      (Variables|Default|SetPathfinderRef _returnvalue))
    (:Is%20Not%20Valid
      (bind _returnvalue_2 (Game|SpawnActorfromClass "/Script/TBS_Project.Pathfinding" (Math|Transform|MakeTransform "0, 0, 0" "0, 0, 0" "1.000000,1.000000,1.000000") "Undefined" 0 0))
      (Variables|Default|SetPathfinderRef _returnvalue_2))))

(fn RemoveHighlightInstances
  (bind _tilehighlightinstancesid (Variables|Default|GetTileHighlightInstancesId))
  (Class|InstancedStaticMeshComponent|RemoveInstances (Variables|/Game/Blueprints/Grid/BP_TileHighlight.BP_TileHighlight_C|GetInstancedHighlight (Variables|Default|GetTileHighlightReference)) _tilehighlightinstancesid)
  (Utilities|Array|Clear _tilehighlightinstancesid))

(fn FindPath
  ;[1 1 1] First find path using C++ A* based pathfinding function
  (Utilities|FlowControl|Sequence
    (:then_0
      (bind _returnvalue (Class|Pathfinding|FindPath (Variables|Default|GetPathfinderRef) (Variables|Default|GetPathfindingStartTileRef) (Variables|Default|GetPathfindingTargetTileRef)))
      (Variables|Default|SetPathFound _returnvalue))
    (:then_1
      ;[1 1 1] Filter array for character movement range that is get from integrated GAS. Also Reverse array since output of C++ function is reversed (from target to start tile)
      (Utilities|Array|Reverse (Variables|Default|GetPathFound))
      (Utilities|Array|Resize (Variables|Default|GetPathFound) (Variables|Default|GetCharacterMovementRange))
      (bind _filteredarray (Utilities|Array|FilterArray (Variables|Default|GetPathFound) "/Script/TBS_Project.TileBase")) ; Filter is done because Resize to movement range could leave empty array elements. So filter removes empty array elements
      (return _filteredarray))))

(fn ClearPath
  (Variables|Default|SetPathfindingStartTileRef 0)
  (Utilities|Array|Clear (Variables|Default|GetPathFound)))