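; Grid actor that generates a tiled room on BeginPlay, using the GameMode's random stream for all random choices.
; GridConstruction rolls a room type and one to four doors, then picks random non-corner door indices and trims them to the door count.
; SpawnGrid then loops over the grid, marks border versus interior tiles, records each in a tile array and adds an instanced static mesh.
; The door indices are not yet applied to the tiles.
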(event EventBeginPlay
  (bind _asbp_game_mode (Utilities|Casting|CastToBP_GameMode (Game|GetGameMode)))
  (Variables|Default|SetGameModeRef _asbp_game_mode)
  (CallFunction|GridConstruction))

(fn ConstructionScript)

(fn RemoveDoorLocations
  (bind _gridtilecount (Variables|Default|GetGridTileCount))
  (bind _returnvalue (- (.y _gridtilecount) 2))
  (bind _returnvalue_2 (- (.x _gridtilecount) 2))
  (bind _output_get (Variables|Default|SetRandomIntArray (Utilities|Array|MakeArray (Math|Random|RandomIntegerinRangefromStream 1 _returnvalue (Variables|/Game/Blueprints/BP_GameMode.BP_GameMode_C|GetStream (Variables|Default|GetGameModeRef))) (Math|Random|RandomIntegerinRangefromStream 1 _returnvalue (Variables|/Game/Blueprints/BP_GameMode.BP_GameMode_C|GetStream (Variables|Default|GetGameModeRef))) (Math|Random|RandomIntegerinRangefromStream 1 _returnvalue_2 (Variables|/Game/Blueprints/BP_GameMode.BP_GameMode_C|GetStream (Variables|Default|GetGameModeRef))) (Math|Random|RandomIntegerinRangefromStream 1 _returnvalue_2 (Variables|/Game/Blueprints/BP_GameMode.BP_GameMode_C|GetStream (Variables|Default|GetGameModeRef))))))
  (for _index (range (.doornumber (Variables|Default|GetfRoomRef)) (Utilities|Array|Length _output_get))
    (Utilities|Array|RemoveIndex (Variables|Default|GetRandomIntArray) (.OutIndex (Utilities|Array|RandomFromStream (Variables|Default|GetRandomIntArray) (Variables|/Game/Blueprints/BP_GameMode.BP_GameMode_C|GetStream (Variables|Default|GetGameModeRef)))))))

(fn MakeRoomStructure
  (bind _gamemoderef (Variables|Default|GetGameModeRef))
  (bind _stream (Variables|/Game/Blueprints/BP_GameMode.BP_GameMode_C|GetStream _gamemoderef))
  (bind _returnvalue (Math|Random|RandomIntegerinRangefromStream 0 3 _stream))
  (Variables|Default|SetfRoomRef (Utilities|Struct|MakeF_Room (Utilities|Enum|ByteToEnumE_RoomTypes (Math|Conversions|ToByte(Integer) _returnvalue)) (+ _returnvalue 1))))

(fn SpawnGrid
  (bind _returnvalue (Transformation|GetActorLocation))
  (bind _gridtilecount (Variables|Default|GetGridTileCount))
  (bind _gridtilecount_2 (Variables|Default|GetGridTileCount))
  (Utilities|Array|Resize (Variables|Default|GetF%20TileArray) (* (.x _gridtilecount) (.y _gridtilecount)))
  (bind (_current_point _total_points _0_1_phase _poly_center _x_row _y_row) (Utilities|2DGridExecutionMacroOwn (Variables|Default|GetGridSnapValue) (Math|Vector|MakeVector (.x _returnvalue) (.y _returnvalue) (- (.z _returnvalue) (/ (Variables|Default|GetGridSnapValue) 2.0))) (.x _gridtilecount_2) (.y _gridtilecount_2))
    (:Per%20Poly%20Execution
      (bind _tiletypeoutput (CallFunction|SetTileType _x_row _y_row _current_point))
      (Utilities|Array|SetArrayElem (Variables|Default|GetF%20TileArray) _current_point (Utilities|Struct|MakeF_Tile _current_point 0 _tiletypeoutput _poly_center))
      (Components|InstancedStaticMesh|AddInstance (Variables|Default|GetInstancedStaticMesh) (Math|Transform|MakeTransform _poly_center "0, 0, 0" "1.000000,1.000000,1.000000") true))))

(fn GridConstruction
  (CallFunction|MakeRoomStructure)
  (CallFunction|RemoveDoorLocations)
  (CallFunction|SpawnGrid))

(fn SetTileType
  (params (X :type Integer) (Y :type Integer) (CurrentPoint :type Integer))
  (bind _gridtilecount (Variables|Default|GetGridTileCount))
  (if (Math|Boolean|ORBoolean (== X 0) (== Y 0) (== (- (.x _gridtilecount) 1) Y) (== X (- (.y _gridtilecount) 1)))
    (return "NewEnumerator1")
    (else
      (return "NewEnumerator0"))))