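; BP_PlayerCamera is a player camera actor that moves on input through a movement component.
; The construction script applies configurable pitch to the camera, with zero roll and yaw in world space, and sets the spring arm's length and socket offset from variables.
; The PlayerMove event maps 2D input onto the actor's forward and right vectors and feeds the result to the movement component.
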(event EventPlayerMove
  (params (MovementInput :type Vector%202D%20Structure))
  (Class|PawnMovementComponent|AddInputVector (Variables|Default|GetMovementComponent) (+ (* (.x MovementInput) (Transformation|GetActorForwardVector)) (* (.y MovementInput) (Transformation|GetActorRightVector))) false))

(fn ConstructionScript
  (bind _springarm (Variables|Default|GetSpringArm))
  (Transformation|SetWorldRotation (Variables|Default|GetCamera) (Math|Rotator|MakeRotator 0.0 (.pitch (Variables|Default|GetCameraRotation)) 0.0) false false)
  (Variables|/Script/Engine.SpringArmComponent|SetTargetArmLength _springarm (Variables|Default|GetTarget%20Arm%20Length))
  (Variables|/Script/Engine.SpringArmComponent|SetSocketOffset _springarm (Variables|Default|GetSocket%20Offset)))