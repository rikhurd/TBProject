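; Base character Blueprint for a tile-based combat game that switches between exploration and combat modes.
; It grants a move ability on BeginPlay and forwards the Interact input to the last overlapped actor through an interface message.
; Combat init halts movement, binds click and overlap events and caches the controller, which is messaged when the character is clicked for selection.
; Exploration init, hover and tile setting are empty, and pathfinding and camera-possession code is disconnected.
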(event Custom|CombatHover
  (params (OverlappedActor :type Actor%20Object%20Reference) (OtherActor :type Actor%20Object%20Reference))
  ;[1 1 1] Grid related functions and events
)

(event Custom|CombatClicked
  (params (TouchedActor :type Actor%20Object%20Reference) (ButtonPressed :type Key%20Structure :default "None"))
  ;[1 1 1] Grid related functions and events
  (CallFunction|SelectCharacter))

(event Input|EnhancedActionEvents|EnhancedInputActionIA_Interact
  (params (ActionValue :type Boolean) (ElapsedSeconds :type Float%20%28double-precision%29) (TriggeredSeconds :type Float%20%28double-precision%29) (InputAction :type Input%20Action%20Object%20Reference :default "/Game/Inputs/Actions/IA_Interact.IA_Interact"))
  (bind _overlappingactorref (Variables|Default|GetOverlappingActorRef))
  ;[1 1 1] Placeholder interact. Used currently for teleporting player to the grid for testing
  (Utilities|IsValid _overlappingactorref
    (:Is%20Valid
      (Class|BPIPlayerInput|PlayerInteract(Message) _overlappingactorref self))))

(event EventCombatModeInit
  ;[1 1 1] Handle game state changes on the character
  (CallFunction|CharacterCombatModeInit))

(event Collision|EventActorBeginOverlap
  (params (OtherActor :type Actor%20Object%20Reference))
  ;[1 1 1] Placeholder interact. Used currently for teleporting player to the grid for testing
  (Variables|Default|SetOverlappingActorRef OtherActor))

(event EventBeginPlay
  ;[1 1 1] PH: Testing move ability. However move ability is going to be on every character
  (GameplayAbilities|GiveAbility (Variables|Default|GetAbilitySystemComponent) "/Game/Blueprints/AbilitySystem/GameplayAbilities/BP_GA_Move.BP_GA_Move_C" 0 -1))

(event Collision|EventActorEndOverlap
  (params (OtherActor :type Actor%20Object%20Reference))
  ;[1 1 1] Placeholder interact. Used currently for teleporting player to the grid for testing
  (Variables|Default|SetOverlappingActorRef 0))

(event EventSetCurrentTile
  (params (Tile :type Tile%20Base%20Object%20Reference))
  ;[1 1 1] Grid related functions and events
)

(event EventExplorationModeInit
  ;[1 1 1] Handle game state changes on the character
  (CallFunction|CharacterExplorationModeInit))

(fn ConstructionScript)

(fn SelectCharacter
  (Development|PrintString (Utilities|GetDisplayName self))
  ;[1 1 1] Interface here that will discuss with character / controller and UI which character is selected
  (Class|BPIPlayerInput|PlayerSelect(Message) (Variables|Default|GetPlayerController) self))

(fn CharacterCombatModeInit
  (bind _returnvalue (Pawn|GetController))
  ;[1 1 1] Set variables that are needed later and setup the start of the combat
  (Components|Movement|StopMovementImmediately (Variables|Character|GetCharacterMovement)) ; Stops animation
  (EventDispatchers|BindEventtoOnClicked (EventDispatchers|CreateEvent :!event Custom|CombatClicked))
  (Collision|BindEventtoOnActorBeginOverlap (EventDispatchers|CreateEvent :!event Custom|CombatHover))
  ;[1 1 1] Since we are about to possess camera pawn set current controller before that
  (Utilities|IsValid _returnvalue
    (:Is%20Valid
      (Variables|Default|SetPlayerController _returnvalue))
    (:Is%20Not%20Valid
      (Development|PrintString "No controller for this character"))))

(fn CharacterExplorationModeInit)