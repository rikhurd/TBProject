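; BP_PlayerCharacter is the player's character Blueprint, handling free movement and the switch to combat mode.
; PlayerMove turns 2D input into movement along the actor's forward and right vectors.
; CharacterCombatModeInit extends its parent by caching the controller, spawning a BP_PlayerCamera from the current camera location, blending the view and possessing it for independent movement.
; PlayerExplorationModeInit is an empty stub.
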(event EventBeginPlay
  (|CallParentFunction) ; This node is disabled and will not be called.\nDrag off pins to build functionality.
)

(event Collision|EventActorBeginOverlap
  (params (OtherActor :type Actor%20Object%20Reference))
  (|CallParentFunction OtherActor) ; This node is disabled and will not be called.\nDrag off pins to build functionality.
)

(event EventTick
  (params (DeltaSeconds :type Float%20%28single-precision%29)))

(event EventPlayerMove
  (params (MovementInput :type Vector%202D%20Structure))
  ;[1 1 1] Player movement in free movement mode
  (Class|PawnMovementComponent|AddInputVector (Variables|Character|GetCharacterMovement) (+ (* (.x MovementInput) (Transformation|GetActorForwardVector)) (* (.y MovementInput) (Transformation|GetActorRightVector))) false))

(fn ConstructionScript
  (|CallParentFunction))

(fn PlayerExplorationModeInit)

(fn PlayerCombatModeInit
  (bind _returnvalue (Pawn|GetController))
  ;[1 1 1] Since we are about to possess camera pawn set current controller before that
  (Variables|Default|SetPlayerController (Pawn|GetController))
  ;[1 1 1] Spawn combat carema for independant movement and possess it
  (bind _returnvalue_2 (Game|SpawnActorfromClass "/Game/Blueprints/Character/BP_PlayerCamera.BP_PlayerCamera_C" (Math|Transform|MakeTransform (Transformation|GetActorLocation) "0, 0, 0" "1.000000,1.000000,1.000000") "Undefined" "MultiplyWithRoot" 0 (Transformation|GetWorldLocation (Variables|Default|GetCamera)) 0))
  (Game|Player|SetViewTargetwithBlend (.AsPlayer%20Controller (Utilities|Casting|CastToPlayerController _returnvalue)) _returnvalue_2 1.0 "VTBlend_EaseIn" 0.4 false)
  (Pawn|Possess _returnvalue _returnvalue_2))

(fn CharacterCombatModeInit
  (|CallParentFunction)
  (CallFunction|PlayerCombatModeInit))